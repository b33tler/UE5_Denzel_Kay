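; VR gun actor that supports one- and two-handed gripping with motion controllers.
; Grab tests controller distance against main and secondary grip spheres, attaching the mesh to the main hand via the GripPoint socket.
; With both hands held, Tick derives roll and yaw from the hand-to-hand look-at, but pitch from the main controller's world X.
; Releasing the main hand detaches the actor; releasing the secondary restores the one-handed transform.
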(event EventRelease
  (params (MotionControllerInput :type Motion%20Controller%20Component%20Object%20Reference))
  (Utilities|FlowControl|Sequence
    (:then_0
      (if (== MotionControllerInput (Variables|Default|GetMainGripController))
        (Variables|Default|SetMainGripController 0)
        (Variables|Default|SetSecondaryGripController 0)
        (Transformation|DetachFromActor "KeepWorld" "KeepWorld" "KeepWorld")))
    (:then_1
      (if (== MotionControllerInput (Variables|Default|GetSecondaryGripController))
        (Variables|Default|SetSecondaryGripController 0)
        (Variables|Default|GetMainGripController
          (:then
            (Transformation|SetActorRelativeTransform (Transformation|GetSocketTransform (Variables|Default|GetSkeletalMesh) "GripPoint" "RTS_Actor") false false))
          (:else
            (Transformation|DetachFromActor "KeepWorld" "KeepWorld" "KeepWorld")))))))

(event EventGrab
  (params (MotionControllerInput :type Motion%20Controller%20Component%20Object%20Reference))
  (bind _maingripcollision (Variables|Default|GetMainGripCollision))
  (bind _secondarygripcollision (Variables|Default|GetSecondaryGripCollision))
  (if (<= (Math|Vector|Distance(Vector) (Transformation|GetWorldLocation MotionControllerInput) (Transformation|GetWorldLocation _maingripcollision)) (Variables|/Script/Engine.SphereComponent|GetSphereRadius _maingripcollision))
    (bind _output_get (Variables|Default|SetMainGripController MotionControllerInput))
    (Transformation|AttachComponentToComponent (Variables|Default|GetSkeletalMesh) _output_get "None" "SnapToTarget" "SnapToTarget" "KeepWorld" true)
    (Transformation|SetActorRelativeTransform (Transformation|GetSocketTransform (Variables|Default|GetSkeletalMesh) "GripPoint" "RTS_Actor") false false)
    (elif (<= (Math|Vector|Distance(Vector) (Transformation|GetWorldLocation MotionControllerInput) (Transformation|GetWorldLocation _secondarygripcollision)) (Variables|/Script/Engine.SphereComponent|GetSphereRadius _secondarygripcollision))
      (Variables|Default|SetSecondaryGripController MotionControllerInput))))

(event EventTick
  (params (DeltaSeconds :type Float%20%28single-precision%29))
  (bind _maingripcontroller (Variables|Default|GetMainGripController))
  (bind _secondarygripcontroller (Variables|Default|GetSecondaryGripController))
  (bind _returnvalue (Transformation|GetWorldLocation _secondarygripcontroller))
  (bind _returnvalue_2 (Transformation|GetWorldLocation _maingripcontroller))
  (bind _returnvalue_3 (Math|Rotator|FindLookatRotation _returnvalue_2 _returnvalue))
  (bind _returnvalue_4 (Math|Rotator|CombineRotators _returnvalue_3 "0.000000,-90.000000,0.000000"))
  (if (and (Utilities|IsValid (Variables|Default|GetMainGripController)) (Utilities|IsValid (Variables|Default|GetSecondaryGripController)))
    (Transformation|SetActorRotation (Math|Rotator|MakeRotator (* (.pitch _returnvalue_4) -1.0) (.x (Transformation|GetWorldLocation _maingripcontroller)) (.yaw _returnvalue_4)))))

(fn ConstructionScript)